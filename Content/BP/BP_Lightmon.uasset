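; BP_Lightmon is a light actor in the Halloween game that flags when a HalloweenCharacter is inside its capsule.
; On BeginPlay, a timeline's vector track drives the LightMon component's rotation through MoveComponentTo, targeting its current world location.
; Capsule overlaps set or clear IsLightBool on HalloweenGameMode.
; Tick polls the game mode's LightDead flag and stops the move when it is true.
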(event OnComponentBeginOverlap(Capsule)
  (params (OverlappedComponent :type Primitive%20Component%20Object%20Reference) (OtherActor :type Actor%20Object%20Reference) (OtherComp :type Primitive%20Component%20Object%20Reference) (OtherBodyIndex :type Integer) (bFromSweep :type Boolean) (SweepResult :type Hit%20Result%20Structure%20%28by%20ref%29))
  (bind _ashalloween_character (Utilities|Casting|CastToHalloweenCharacter OtherActor))
  (bind _ashalloween_game_mode (Utilities|Casting|CastToHalloweenGameMode (Game|GetGameMode)))
  (Variables|/Game/SideScrollerBP/Blueprints/HalloweenGameMode.HalloweenGameMode_C|SetisLightBool _ashalloween_game_mode true))

(event OnComponentEndOverlap(Capsule)
  (params (OverlappedComponent :type Primitive%20Component%20Object%20Reference) (OtherActor :type Actor%20Object%20Reference) (OtherComp :type Primitive%20Component%20Object%20Reference) (OtherBodyIndex :type Integer))
  (bind _ashalloween_character (Utilities|Casting|CastToHalloweenCharacter OtherActor))
  (bind _ashalloween_game_mode (Utilities|Casting|CastToHalloweenGameMode (Game|GetGameMode)))
  (Variables|/Game/SideScrollerBP/Blueprints/HalloweenGameMode.HalloweenGameMode_C|SetisLightBool _ashalloween_game_mode false))

(event EventBeginPlay
  (bind _lightmon (Variables|Default|GetLightMon))
  (bind _새_트랙_0 (Timeline|Light Play)
    (:Update
      (Components|MoveComponentTo _lightmon (Transformation|GetWorldLocation _lightmon) (Math|Conversions|RotationFromXVector _새_트랙_0) false false 1e+01 false))))

(event EventTick
  (params (DeltaSeconds :type Float%20%28single-precision%29))
  (bind _lightmon (Variables|Default|GetLightMon))
  (bind _ashalloween_game_mode (Utilities|Casting|CastToHalloweenGameMode (Game|GetGameMode)))
  (if (Variables|/Game/SideScrollerBP/Blueprints/HalloweenGameMode.HalloweenGameMode_C|GetLightDead _ashalloween_game_mode)
    (Components|MoveComponentTo _lightmon (Transformation|GetWorldLocation _lightmon) (Math|Conversions|RotationFromXVector (stale EventBeginPlay _새_트랙_0)) false false 1e+01 false) ; enters at Stop
  ))

(fn ConstructionScript)