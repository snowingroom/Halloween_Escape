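; BP_Animal is an enemy pawn that chases the player and damages them on contact.
; It loops a crawl animation and, after a one-second timer, runs a Move event that re-issues AI MoveTo toward the player on success or failure.
; Capsule hits from HalloweenCharacter pass through HitDelay, a hit counter that throttles damage to every HitCompleteNum hits instead of using a timed delay.
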(event OnComponentHit(CapsuleComponent)
  (params (HitComponent :type Primitive%20Component%20Object%20Reference) (OtherActor :type Actor%20Object%20Reference) (OtherComp :type Primitive%20Component%20Object%20Reference) (NormalImpulse :type Vector :default "0, 0, 0") (Hit :type Hit%20Result%20Structure%20%28by%20ref%29))
  (Utilities|Casting|CastToHalloweenCharacter OtherActor)
  (|HitDelay)
  (Game|Damage|ApplyDamage (Game|GetPlayerCharacter 0) 1e+01 (Game|GetInstigatorController) self))

(event Custom|Move
  (bind _returnvalue (Game|GetPlayerCharacter 0))
  (AI|AIMoveTo self (Transformation|GetActorLocation _returnvalue) _returnvalue 5.0 false
    (:OnSuccess
      _)
    (:OnFail
      _))
  (CallFunction|Move))

(event EventBeginPlay
  (Components|Animation|PlayAnimation (Variables|Character|GetMesh) "/Game/Source/Animal/running_crawl_inPlace_Anim_mixamo_com.running_crawl_inPlace_Anim_mixamo_com" true)
  (Utilities|Time|SetTimerbyFunctionName 0 "Move" 1.0))

(fn ConstructionScript)