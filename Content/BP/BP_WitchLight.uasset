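; BP_WitchLight is the witch's house trigger in a Halloween game, with a light that signals whether entry is safe.
; Tick hides the PointLight whenever the GameMode's IsWitchNaGam (witch is out) flag is set.
; Entering HouseZon then teleports the character to NewLocetion after a delay.
; Otherwise it sets IsDead, hides the light, then after a delay shows particles, disables input and damages the player.
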(event OnComponentBeginOverlap(HouseZon)
  (params (OverlappedComponent :type Primitive%20Component%20Object%20Reference) (OtherActor :type Actor%20Object%20Reference) (OtherComp :type Primitive%20Component%20Object%20Reference) (OtherBodyIndex :type Integer) (bFromSweep :type Boolean) (SweepResult :type Hit%20Result%20Structure%20%28by%20ref%29))
  (bind _ashalloween_character (Utilities|Casting|CastToHalloweenCharacter OtherActor))
  (bind _ashalloween_game_mode (Utilities|Casting|CastToHalloweenGameMode (Game|GetGameMode)))
  (if (Variables|/Game/SideScrollerBP/Blueprints/HalloweenGameMode.HalloweenGameMode_C|GetisWitchNaGam _ashalloween_game_mode)
    (Utilities|FlowControl|Delay 1.0)
    (Transformation|SetActorLocation _ashalloween_character (Variables|Default|GetNewLocetion) false true)
    (else
      (Variables|/Game/SideScrollerBP/Blueprints/HalloweenGameMode.HalloweenGameMode_C|SetisDead _ashalloween_game_mode true)
      (Rendering|SetVisibility (Variables|Default|GetPointLight) false false)
      (Utilities|FlowControl|Delay 1.0)
      (Rendering|SetVisibility (Variables|Default|GetParticleSystem) true false)
      (Input|DisableInput _ashalloween_game_mode 0)
      (Game|Damage|ApplyDamage (Game|GetPlayerCharacter 0) (Variables|Default|GetDamagePoint) (Game|GetInstigatorController) self))))

(event EventBeginPlay)

(event Collision|EventActorBeginOverlap
  (params (OtherActor :type Actor%20Object%20Reference)))

(event EventTick
  (params (DeltaSeconds :type Float%20%28single-precision%29))
  (bind _ashalloween_game_mode (Utilities|Casting|CastToHalloweenGameMode (Game|GetGameMode)))
  (if (Variables|/Game/SideScrollerBP/Blueprints/HalloweenGameMode.HalloweenGameMode_C|GetisWitchNaGam _ashalloween_game_mode)
    (Rendering|SetVisibility (Variables|Default|GetPointLight) false false)))

(fn ConstructionScript)