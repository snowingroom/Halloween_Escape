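; BP_WitchStartZon is a trigger zone that starts the witch encounter when the player's HalloweenCharacter enters its Box.
; After a WitchZonStartTime delay, it checks that the HalloweenGameMode does not report the player as dead.
; It then sets the game mode's IsWitchNaGam flag and spawns BP_Witch at WitchPosition.
; Nothing in the graph disables the trigger after it fires.
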(event OnComponentBeginOverlap(Box)
  (params (OverlappedComponent :type Primitive%20Component%20Object%20Reference) (OtherActor :type Actor%20Object%20Reference) (OtherComp :type Primitive%20Component%20Object%20Reference) (OtherBodyIndex :type Integer) (bFromSweep :type Boolean) (SweepResult :type Hit%20Result%20Structure%20%28by%20ref%29))
  (Utilities|Casting|CastToHalloweenCharacter OtherActor)
  (Utilities|FlowControl|Delay (Variables|Default|GetWitchZonStartTime))
  (bind _ashalloween_game_mode (Utilities|Casting|CastToHalloweenGameMode (Game|GetGameMode)))
  (if (not (Variables|/Game/SideScrollerBP/Blueprints/HalloweenGameMode.HalloweenGameMode_C|GetisDead _ashalloween_game_mode))
    (Variables|/Game/SideScrollerBP/Blueprints/HalloweenGameMode.HalloweenGameMode_C|SetisWitchNaGam _ashalloween_game_mode true)
    (Game|SpawnActorfromClass "/Game/BP/BP_Witch.BP_Witch_C" (Math|Conversions|ToTransform(Vector) (Variables|Default|GetWitchPosition)) "Undefined" 0 0)))

(event EventBeginPlay)

(event Collision|EventActorBeginOverlap
  (params (OtherActor :type Actor%20Object%20Reference)))

(event EventTick
  (params (DeltaSeconds :type Float%20%28single-precision%29)))

(fn ConstructionScript)