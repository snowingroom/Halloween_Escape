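; BP_LampPlace is a lamp trigger actor that sets the lamp item flag on HalloweenGameMode when the player character reaches it.
; Entering its Sphere turns on PointLight1, then after a short delay sets IsLampItem and destroys the actor.
; Leaving turns the light off but does not cancel the delay.
; Tick debug-prints the character's IsHand and latches ITemSkill when true, though nothing here reads it.
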(event OnComponentBeginOverlap(Sphere)
  (params (OverlappedComponent :type Primitive%20Component%20Object%20Reference) (OtherActor :type Actor%20Object%20Reference) (OtherComp :type Primitive%20Component%20Object%20Reference) (OtherBodyIndex :type Integer) (bFromSweep :type Boolean) (SweepResult :type Hit%20Result%20Structure%20%28by%20ref%29))
  (bind _ashalloween_character (Utilities|Casting|CastToHalloweenCharacter OtherActor))
  (Rendering|SetVisibility (Variables|Default|GetPointLight1) true false)
  (Utilities|FlowControl|Delay 2.0)
  (bind _ashalloween_game_mode (Utilities|Casting|CastToHalloweenGameMode (Game|GetGameMode)))
  (Variables|/Game/SideScrollerBP/Blueprints/HalloweenGameMode.HalloweenGameMode_C|SetisLampItem _ashalloween_game_mode true)
  (Actor|DestroyActor))

(event OnComponentEndOverlap(Sphere)
  (params (OverlappedComponent :type Primitive%20Component%20Object%20Reference) (OtherActor :type Actor%20Object%20Reference) (OtherComp :type Primitive%20Component%20Object%20Reference) (OtherBodyIndex :type Integer))
  (Utilities|Casting|CastToHalloweenCharacter OtherActor)
  (Rendering|SetVisibility (Variables|Default|GetPointLight1) false false))

(event EventBeginPlay)

(event Collision|EventActorBeginOverlap
  (params (OtherActor :type Actor%20Object%20Reference)))

(event EventTick
  (params (DeltaSeconds :type Float%20%28single-precision%29))
  (bind _ashalloween_character (Utilities|Casting|CastToHalloweenCharacter (Game|GetPlayerCharacter 0)))
  (Development|PrintString (Utilities|String|ToString(Boolean) (Variables|/Game/SideScrollerBP/Blueprints/HalloweenCharacter.HalloweenCharacter_C|GetIsHand _ashalloween_character)) false)
  (if (Variables|/Game/SideScrollerBP/Blueprints/HalloweenCharacter.HalloweenCharacter_C|GetIsHand _ashalloween_character)
    (Variables|Default|SetITemSkill true)))

(fn ConstructionScript)