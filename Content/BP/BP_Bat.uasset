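; BP_Bat is a moving bat hazard that knocks back and damages the player on contact.
; Six bat meshes loop one animation, while a timeline started on BeginPlay feeds offsets from the initial location into MoveComponentTo on the capsule.
; Capsule overlap with a HalloweenCharacter launches it along fixed world +Y, then applies DamagePoint damage to player character 0 rather than the overlapping actor reference.
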(event OnComponentBeginOverlap(CapsuleComponent)
  (params (OverlappedComponent :type Primitive%20Component%20Object%20Reference) (OtherActor :type Actor%20Object%20Reference) (OtherComp :type Primitive%20Component%20Object%20Reference) (OtherBodyIndex :type Integer) (bFromSweep :type Boolean) (SweepResult :type Hit%20Result%20Structure%20%28by%20ref%29))
  (bind _ashalloween_character (Utilities|Casting|CastToHalloweenCharacter OtherActor))
  (Character|LaunchCharacter _ashalloween_character "0.000000,300.000000,0.000000" true false)
  (CallFunction|Damage))

(event Custom|Damage
  (Game|Damage|ApplyDamage (Game|GetPlayerCharacter 0) (Variables|Default|GetDamagePoint) (Game|GetInstigatorController) self))

(event EventBeginPlay
  (Components|Animation|PlayAnimation (Variables|Character|GetMesh) "/Game/Source/Bat/BatExample_Anim_mixamo_com.BatExample_Anim_mixamo_com" true)
  (Variables|Default|SetIniLocation (Transformation|GetWorldLocation (Variables|Collision|GetCapsuleComponent)))
  (bind _새_트랙_0 (Timeline|BatMovement1 Play)
    (:Update
      (Components|MoveComponentTo (Variables|Collision|GetCapsuleComponent) (+ (Variables|Default|GetIniLocation) _새_트랙_0) "0, 0, 0" false false 5.0 false))))

(fn ConstructionScript)