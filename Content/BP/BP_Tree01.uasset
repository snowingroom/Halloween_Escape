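; BP_Tree01 is a tree that rotates through five stages, apparently being chopped down, while the side-scroller player's IsHand flag is set.
; Tick reads and debug-prints that flag, then switches on AxCount to pick the next target rotation.
; MoveComponentTo animates the mesh, with a slower final stage, and TreeCount then increments AxCount.
; The mesh's world location is passed as the relative location target.
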(event Custom|TREE)

(event EventTick
  (params (DeltaSeconds :type Float%20%28single-precision%29))
  (bind _staticmeshcomponent (Variables|Debug|GetStaticMeshComponent))
  (bind _staticmeshcomponent_2 (Variables|Debug|GetStaticMeshComponent))
  (bind _staticmeshcomponent_3 (Variables|Debug|GetStaticMeshComponent))
  (bind _staticmeshcomponent_4 (Variables|Debug|GetStaticMeshComponent))
  (bind _staticmeshcomponent_5 (Variables|Debug|GetStaticMeshComponent))
  (bind _asside_scroller_character (Utilities|Casting|CastToSideScrollerCharacter (Game|GetPlayerCharacter 0)))
  (Development|PrintString (Utilities|String|ToString(Boolean) (Variables|/Game/SideScrollerBP/Blueprints/SideScrollerCharacter.SideScrollerCharacter_C|GetIsHand _asside_scroller_character)))
  (if (Variables|/Game/SideScrollerBP/Blueprints/SideScrollerCharacter.SideScrollerCharacter_C|GetIsHand _asside_scroller_character)
    (switch int (Variables|Default|GetAxCount)
      (:0
        (Components|MoveComponentTo _staticmeshcomponent_2 (Transformation|GetWorldLocation _staticmeshcomponent_2) (Variables|Default|GetRotation1) false false 0.5 true))
      (:1
        (Components|MoveComponentTo _staticmeshcomponent_3 (Transformation|GetWorldLocation _staticmeshcomponent_3) (Variables|Default|GetRotaton2) false false 0.5 true))
      (:2
        (Components|MoveComponentTo _staticmeshcomponent_4 (Transformation|GetWorldLocation _staticmeshcomponent_4) (Variables|Default|GetRotation3) false false 0.5 true))
      (:3
        (Components|MoveComponentTo _staticmeshcomponent_5 (Transformation|GetWorldLocation _staticmeshcomponent_5) (Variables|Default|GetRotation4) false false 0.5 true))
      (:4
        (Components|MoveComponentTo _staticmeshcomponent (Transformation|GetWorldLocation _staticmeshcomponent) (Variables|Default|GetRotationFinal) false false 2.0 true)))
    (CallFunction|TreeCount)))

(fn ConstructionScript)

(fn TreeCount
  (Variables|Default|SetAxCount (+ 1 (Variables|Default|GetAxCount))))